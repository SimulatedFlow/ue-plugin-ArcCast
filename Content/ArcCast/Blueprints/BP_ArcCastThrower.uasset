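; BP_ArcCastThrower is an ArcCast test thrower that switches between preset shots, arc profiles and manual aim.
; Shot events set the index, pitch and yaw, then apply rotation and launch speed override to the ArcCast component.
; Profile events swap grenade, teleport, arrow or bouncy data assets.
; Aim events step the stored angles, but the applied rotation adds the step again, running one step ahead of the variables.
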(event `self.ReceiveBeginPlay`
  (bind _arccast (`self.ArcCast`))
  (set `self.ShotIndex` 0)
  (set `self.ProfileIndex` 0)
  (set `self.AimPitch` 35.0)
  (set `self.AimYaw` 0.0)
  (`ArcCastComponent.SetProfile` _arccast "/ArcCast/ArcCast/Profiles/DA_Arc_Grenade.DA_Arc_Grenade")
  (`ArcCastComponent.SetLaunchSpeedOverride` _arccast 0.0)
  (`SceneComponent.K2_SetRelativeRotation` _arccast (`KismetMathLibrary.MakeRotator` 0.0 35.0) false false))

(event `ShotLandingPad`
  (bind _arccast (`self.ArcCast`))
  (set `self.ShotIndex` 0)
  (set `self.AimPitch` 35.0)
  (set `self.AimYaw` 0.0)
  (`ArcCastComponent.SetLaunchSpeedOverride` _arccast 0.0)
  (`SceneComponent.K2_SetRelativeRotation` _arccast (`KismetMathLibrary.MakeRotator` 0.0 35.0) false false))

(event `ShotStairs`
  (bind _arccast (`self.ArcCast`))
  (set `self.ShotIndex` 1)
  (set `self.AimPitch` 45.0)
  (set `self.AimYaw` -17.0)
  (`ArcCastComponent.SetLaunchSpeedOverride` _arccast 0.0)
  (`SceneComponent.K2_SetRelativeRotation` _arccast (`KismetMathLibrary.MakeRotator` 0.0 45.0 -17.0) false false))

(event `ShotSteepRamp`
  (bind _arccast (`self.ArcCast`))
  (set `self.ShotIndex` 2)
  (set `self.AimPitch` 45.0)
  (set `self.AimYaw` 26.0)
  (`ArcCastComponent.SetLaunchSpeedOverride` _arccast 1450.0)
  (`SceneComponent.K2_SetRelativeRotation` _arccast (`KismetMathLibrary.MakeRotator` 0.0 45.0 26.0) false false))

(event `ShotOverTheLedge`
  (bind _arccast (`self.ArcCast`))
  (set `self.ShotIndex` 3)
  (set `self.AimPitch` 38.0)
  (set `self.AimYaw` -10.0)
  (`ArcCastComponent.SetLaunchSpeedOverride` _arccast 1800.0)
  (`SceneComponent.K2_SetRelativeRotation` _arccast (`KismetMathLibrary.MakeRotator` 0.0 38.0 -10.0) false false))

(event `ProfileGrenade`
  (set `self.ProfileIndex` 0)
  (`ArcCastComponent.SetProfile` (`self.ArcCast`) "/ArcCast/ArcCast/Profiles/DA_Arc_Grenade.DA_Arc_Grenade"))

(event `ProfileTeleport`
  (set `self.ProfileIndex` 1)
  (`ArcCastComponent.SetProfile` (`self.ArcCast`) "/ArcCast/ArcCast/Profiles/DA_Arc_Teleport.DA_Arc_Teleport"))

(event `ProfileArrow`
  (set `self.ProfileIndex` 2)
  (`ArcCastComponent.SetProfile` (`self.ArcCast`) "/ArcCast/ArcCast/Profiles/DA_Arc_Arrow.DA_Arc_Arrow"))

(event `ProfileBouncy`
  (set `self.ProfileIndex` 3)
  (`ArcCastComponent.SetProfile` (`self.ArcCast`) "/ArcCast/ArcCast/Profiles/DA_Arc_Bouncy.DA_Arc_Bouncy"))

(event `AimUp`
  (bind _returnvalue (+ (`self.AimPitch`) 3.0))
  (bind _returnvalue_2 (+ (`self.AimYaw`) 0.0))
  (set `self.AimPitch` _returnvalue)
  (set `self.AimYaw` _returnvalue_2)
  (`SceneComponent.K2_SetRelativeRotation` (`self.ArcCast`) (`KismetMathLibrary.MakeRotator` 0.0 _returnvalue _returnvalue_2) false false))

(event `AimDown`
  (bind _returnvalue (+ (`self.AimPitch`) -3.0))
  (bind _returnvalue_2 (+ (`self.AimYaw`) 0.0))
  (set `self.AimPitch` _returnvalue)
  (set `self.AimYaw` _returnvalue_2)
  (`SceneComponent.K2_SetRelativeRotation` (`self.ArcCast`) (`KismetMathLibrary.MakeRotator` 0.0 _returnvalue _returnvalue_2) false false))

(event `AimLeft`
  (bind _returnvalue (+ (`self.AimPitch`) 0.0))
  (bind _returnvalue_2 (+ (`self.AimYaw`) -5.0))
  (set `self.AimPitch` _returnvalue)
  (set `self.AimYaw` _returnvalue_2)
  (`SceneComponent.K2_SetRelativeRotation` (`self.ArcCast`) (`KismetMathLibrary.MakeRotator` 0.0 _returnvalue _returnvalue_2) false false))

(event `AimRight`
  (bind _returnvalue (+ (`self.AimPitch`) 0.0))
  (bind _returnvalue_2 (+ (`self.AimYaw`) 5.0))
  (set `self.AimPitch` _returnvalue)
  (set `self.AimYaw` _returnvalue_2)
  (`SceneComponent.K2_SetRelativeRotation` (`self.ArcCast`) (`KismetMathLibrary.MakeRotator` 0.0 _returnvalue _returnvalue_2) false false))

(fn `UserConstructionScript`)